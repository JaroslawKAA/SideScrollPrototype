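; AI controller for the melee enemy: runs its behavior tree and performs its combat actions.
; Pawn sensing stores any seen attack target; attacks play a montage when in range, with damage applied on an anim notify after rechecking distance.
; Defense, block and dodge montages set state flags, and dispatchers report attack and defense outcomes.
; The attack reaction alternates between Move Back and Defense, though the MoveBack event is empty.
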(event `self.ReceiveBeginPlay`
  ;[1 1 1] BeginePlay
  (bind _asbp_enemy (cast `/Game/Blueprints/Enemy/BP_Enemy` (`self.K2_GetPawn`)))
  (set `self.BP Enemy` _asbp_enemy)
  (`self.RunBehaviorTree` "/Game/Blueprints/Enemy/AI/BP_EnemyIA.BP_EnemyIA"))

(event `self.PawnSensing.OnSeePawn`
  (params (Pawn :type "Pawn Object Reference"))
  ;[1 1 1] OnSeePawn
  (bind _asbpi_attack_target (cast `/Game/Blueprints/Core/Interfaces/BPI_AttackTarget` Pawn))
  (set `self.AttackTarget` _asbpi_attack_target)
  (set `self.HasSeenPlayer` true))

(event `AttackPlayer`
  ;[1 1 1] Attack Player
  (bind _actor (`/Game/Blueprints/Core/Interfaces/BPI_AttackTarget.AttackTargetActor` (`self.AttackTarget`)))
  (if (< (`KismetMathLibrary.Vector_Distance` (`self.K2_GetActorLocation` _actor) (`self.K2_GetActorLocation` (`self.BP Enemy`))) (`self.AttackRange`))
    (`KismetSystemLibrary.PrintString` "[Enemy] Attack Started")
    (`|PlayMontage` (`Character.Mesh` (`self.BP Enemy`)) "/Game/Mixamo/Animations/StandingMeleeAttackHorizontal_UE_Montage.StandingMeleeAttackHorizontal_UE_Montage"
      (:`OnCompleted`
        (`self.OnAttackEnd`))
      (:`OnInterrupted`
        (`self.OnAttackNotExecuted`)))
    (else
      (`self.OnAttackNotExecuted`))))

(event `/Game/Blueprints/Core/Interfaces/BPI_OnApplyDamageAnimNotify.OnApplyDamageAnimNotice`
  ;[1 1 1] Anim notify subscriber
  ;[1 1 1] ApplyDamage
  (bind _actor (`/Game/Blueprints/Core/Interfaces/BPI_AttackTarget.AttackTargetActor` (`self.AttackTarget`)))
  (if (< (`self.GetDistanceTo` _actor (`self.BP Enemy`)) (`self.AttackRange`))
    (bind _actor_2 (`/Game/Blueprints/Core/Interfaces/BPI_AttackTarget.AttackTargetActor` (`self.AttackTarget`)))
    (`GameplayStatics.ApplyDamage` _actor_2 10.0 null (`self.BP Enemy`))))

(event `Defense`
  ;[1 1 1] Defense
  (`KismetSystemLibrary.PrintString` "[Enemy] Start Defense")
  (`|PlayMontage` (`Character.Mesh` (`self.BP Enemy`)) "/Game/Mixamo/Animations/StandingBlockIdle_UE_Montage.StandingBlockIdle_UE_Montage"
    (:`then`
      (set `self.IsDefense` true))
    (:`OnCompleted`
      (if (not (`self.BlockedAttack`)) :!label _label
        (set `self.IsDefense` false)
        (`self.OnDefenceEndEvent`)))
    (:`OnBlendOut`
      (goto _label))))

(event `BlockAttack`
  (`|PlayMontage` (`Character.Mesh` (`self.BP Enemy`)) "/Game/Mixamo/Animations/StandingBlockReactLarge_UE_Montage.StandingBlockReactLarge_UE_Montage"
    (:`then`
      (set `self.BlockedAttack` true))
    (:`OnCompleted`
      (set `self.BlockedAttack` false)
      (set `self.IsDefense` false)
      (`self.OnDefenceEndEvent`))))

(event `Dodge`
  (`|PlayMontage` (`Character.Mesh` (`self.BP Enemy`)) "/Game/Mixamo/Animations/StandingReactLargeFromLeft_UE_Montage.StandingReactLargeFromLeft_UE_Montage"
    (:`then`
      (set `self.IsDodge` true))
    (:`OnCompleted`
      (set `self.IsDodge` false :!label _label_2))
    (:`OnBlendOut`
      (goto _label_2))
    (:`OnInterrupted`
      (goto _label_2))))

(event `OnAttackEnd_Event`)

(event `MoveBack`)

(event `OnDefenceEndEvent`
  (`self.OnDefenceEnd`))

(event `OnDefenceNotExecuted_Event`)

(event `OnMovedBack`)

(fn `GetAttackReaction`
  (returns (AttackReactionType :type "/Game/Blueprints/Enemy/AI/BPE_AttackReactionType Enum"))
  (return (`self.AttackReactionType`)))

(fn `NextAttackReaction`
  (locals (NewEnumValue :type Integer64))
  (switch `/Game/Blueprints/Enemy/AI/BPE_AttackReactionType` (`self.AttackReactionType`)
    (:`NewEnumerator0`
      (set `self.AttackReactionType` "NewEnumerator1"))
    (:`NewEnumerator1`
      (set `self.AttackReactionType` "NewEnumerator0"))))

(fn `UserConstructionScript`)
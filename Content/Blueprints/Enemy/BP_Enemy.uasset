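; BP_Enemy is an AI-driven enemy character built on a parent class that it extends.
; On BeginPlay it sets walk speed from MaxSpeed and caches its BP_AIController_Enemy.
; Any damage it receives is routed to that controller, which blocks when IsDefense is set and dodges otherwise.
; Tick, Init and the damage anim-notify event only pass through to the parent.
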(event `self.ReceiveBeginPlay`
  (`parent.ReceiveBeginPlay`)
  (set `CharacterMovementComponent.MaxWalkSpeed` (`self.MaxSpeed`) (`self.CharacterMovement`))
  (bind _asbp_aicontroller_enemy (cast `/Game/Blueprints/Enemy/AI/BP_AIController_Enemy` (`AIBlueprintHelperLibrary.GetAIController` self)))
  (set `self.AIController Enemy` _asbp_aicontroller_enemy))

(event `self.ReceiveTick`
  (params (DeltaSeconds :type "Float (single-precision)"))
  (`parent.ReceiveTick` DeltaSeconds))

(event `/Game/Blueprints/Core/Interfaces/BPI_OnApplyDamageAnimNotify.OnApplyDamageAnimNotice`
  (`parent.OnApplyDamageAnimNotice`))

(event `self.ReceiveAnyDamage`
  (params (Damage :type "Float (single-precision)") (DamageType :type "DamageType Object Reference") (InstigatedBy :type "Controller Object Reference") (DamageCauser :type "Actor Object Reference"))
  ;[1 1 1] AnyDamage
  (if (`/Game/Blueprints/Enemy/AI/BP_AIController_Enemy.IsDefense` (`self.AIController Enemy`))
    (`/Game/Blueprints/Enemy/AI/BP_AIController_Enemy.BlockAttack` (`self.AIController Enemy`))
    (else
      (`/Game/Blueprints/Enemy/AI/BP_AIController_Enemy.Dodge` (`self.AIController Enemy`)))))

(event `/Game/Blueprints/Core/Interfaces/BPI_Initiable.Init`
  (`parent.Init`))

(fn `UserConstructionScript`)
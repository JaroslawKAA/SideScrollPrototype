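; Base character Blueprint providing health, stamina, lives, base damage and attack-target getters, with empty events as hooks.
; Init caches the ABP_Manny instance, and Tick pushes velocity, movement and falling state into it directly.
; Stamina drains while moving and regenerates otherwise, with clamped setters raising change events.
; Depleted health refills and costs a life, and a dodge montage reports completion or interruption through events.
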(event `self.ReceiveBeginPlay`
  (if (not (`self.Inited`))
    (`self.Init`)))

(event `self.ReceiveTick`
  (params (DeltaSeconds :type "Float (single-precision)"))
  (if (`/Game/Characters/Mannequins/Animations/ABP_Manny.ShouldMove` (`self.AnimInstance`))
    (`self.LocomotionConsumeStamina` DeltaSeconds)
    (else
      (`self.RegenerateStamina` DeltaSeconds)))
  (`self.ControllAnimations`))

(event `/Game/Blueprints/Core/Interfaces/BPI_Initiable.Init`
  (if (not (`self.Inited`))
    (set `self.Inited` true)
    (bind _asabp_manny (cast `/Game/Characters/Mannequins/Animations/ABP_Manny` (`SkeletalMeshComponent.GetAnimInstance` (`self.Mesh`))))
    (set `self.AnimInstance` _asabp_manny)))

(event `/Game/Blueprints/Core/Interfaces/BPI_OnApplyDamageAnimNotify.OnApplyDamageAnimNotice`)

(event `OnHealthChanged`
  (params (Health :type "Float (double-precision)"))
  (if (<= Health 0.0)
    (`self.SetHealth` (`self.MaxHealth`))
    (bind _result (`/Engine/EditorBlueprintResources/StandardMacros.DecrementInt` (`self.Lifes`))
      (:`  `
        (`self.SetLifes` _result)))))

(event `OnStaminaChanged`)

(event `OnLifesChanged`
  (params (Lifes :type Integer)))

(event `PlayMontageDodge`
  (`|PlayMontage` (`self.Mesh`) "/Game/Mixamo/Animations/StandingReactLargeFromLeft_UE_Montage.StandingReactLargeFromLeft_UE_Montage"
    (:`OnCompleted`
      (`self.DodgeCompleated`))
    (:`OnBlendOut`
      (`self.DodgeNotCompleated` :!label _label))
    (:`OnInterrupted`
      (goto _label))))

(event `DodgeCompleated`)

(event `DodgeNotCompleated`)

(fn `AttackTargetActor`
  (returns (Actor :type "Actor Object Reference"))
  (return self))

(fn `AttackTargetState`
  (returns (AttackTargetState :type "/Game/Blueprints/Core/Enums/AttackTargetState Enum"))
  (return (`self.m_AttackTargetState`)))

(fn `ControllAnimations`
  (`|ExecutionSequence`
    (:`then_0`
      ;[1 1 1] Set velocity and ground speed from the movement components velocity. Ground speed is calculated from only the X and Y axis of the velocity, so moving up or down does not affect it.
      (bind _output_get (set `/Game/Characters/Mannequins/Animations/ABP_Manny.Velocity` (`MovementComponent.Velocity` (`self.CharacterMovement`)) (`self.AnimInstance`)))
      (set `/Game/Characters/Mannequins/Animations/ABP_Manny.GroundSpeed` (`KismetMathLibrary.VSizeXY` _output_get) (`self.AnimInstance`)))
    (:`then_1`
      ;[1 1 1] Set Should Move to true only if ground speed is above a small threshold (to prevent incredibly small velocities from triggering animations) and if there is currently acceleration (input) applied.
      (set `/Game/Characters/Mannequins/Animations/ABP_Manny.ShouldMove` (and (> (`/Game/Characters/Mannequins/Animations/ABP_Manny.GroundSpeed` (`self.AnimInstance`)) 3.0) (!= (`MovementComponent.Velocity` (`self.CharacterMovement`)) (0.0 0.0 0.0))) (`self.AnimInstance`)))
    (:`then_2`
      ;[1 1 1] Set Is Falling from the movement components falling state.
      (set `/Game/Characters/Mannequins/Animations/ABP_Manny.IsFalling` (`NavMovementComponent.IsFalling` (`self.CharacterMovement`)) (`self.AnimInstance`)))))

(fn `GetBaseDamage`
  (returns (BaseDamage :type "Float (double-precision)"))
  (return (`self.BaseDamage`)))

(fn `GetHealth`
  (returns (Health :type "Float (double-precision)"))
  (return (`self.Health`)))

(fn `GetInited`
  (returns (Inited :type Boolean))
  (return (`self.Inited`)))

(fn `GetLifes`
  (returns (Lifes :type Integer))
  (return (`self.Lifes`)))

(fn `GetStamina`
  (returns (Stamina :type "Float (double-precision)"))
  (return (`self.Stamina`)))

(fn `LocomotionConsumeStamina`
  (params (DeltaSeconds :type "Float (double-precision)"))
  (`self.SetStamina` (- (`self.Stamina`) (* DeltaSeconds (`self.StaminaLocomotionConsumption`)))))

(fn `RegenerateStamina`
  (params (DeltaSeconds :type "Float (double-precision)"))
  (`self.SetStamina` (+ (* DeltaSeconds (`self.StaminaRegenerationSpeed`)) (`self.Stamina`))))

(fn `SetHealth`
  (params (Health :type "Float (double-precision)"))
  (bind _output_get (set `self.Health` (`KismetMathLibrary.FClamp` Health 0.0 (`self.MaxHealth`))))
  (`self.OnHealthChanged` _output_get))

(fn `SetLifes`
  (params (Lifes :type Integer))
  (bind _output_get (set `self.Lifes` Lifes))
  (`self.OnLifesChanged` _output_get))

(fn `SetStamina`
  (params (Stamina :type "Float (double-precision)"))
  (set `self.Stamina` (`KismetMathLibrary.FClamp` Stamina 0.0 (`self.MaxStamina`)))
  (`self.OnStaminaChanged`)
  (return))

(fn `UserConstructionScript`)
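; Debug drawing utility functions for visualizing vectors and splines in the world.
; DebugVector draws an orange arrow from a location along the given vector, scaled up by a fixed factor for visibility.
; DebugSpline walks the spline's length in caller-set distance steps, sampling world-space points and joining them with grey debug lines to approximate the curve.
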(fn `DebugSpline`
  (params (WorldContextObject :type "Object Object Reference") (Spline :type "SplineComponent Object Reference") (lineDistances :type "Float (double-precision)"))
  (locals (CurrentSplineDistance :type "Float (double-precision)"))
  (bind _returnvalue (+ (`local.CurrentSplineDistance`) (`local.lineDistances`)))
  (while (< (`local.CurrentSplineDistance`) (`SplineComponent.GetSplineLength` Spline))
    (`KismetSystemLibrary.DrawDebugLine` (`local.WorldContextObject`) (`SplineComponent.GetLocationAtDistanceAlongSpline` (`local.Spline`) (`local.CurrentSplineDistance`) "World") (`SplineComponent.GetLocationAtDistanceAlongSpline` (`local.Spline`) _returnvalue "World") (struct :`R` 0.5 :`G` 0.5 :`B` 0.5 :`A` 1.0) 0.0 3.0)
    (set `local.CurrentSplineDistance` _returnvalue))
  (return))

(fn `DebugVector`
  (params (Vector :type "Vector Structure") (Location :type "Vector Structure"))
  (`KismetSystemLibrary.DrawDebugArrow` null Location (+ (* Vector 100.0) Location) 10.0 (struct :`R` 0.947307 :`G` 0.55834 :`B` 0.015996 :`A` 1.0) 0.0 2.0))
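; BP_TPPGameState is a game state machine state that shows the HUD while it is active.
; Init creates a BP_HUD widget through the PlayerController, stores it and hands it to the GameStateMachine.
; OnEnter adds the HUD to the player screen and OnExit removes it, each after calling the parent implementation.
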(fn `Init`
  (`parent.Init`)
  (bind _result (`/Game/Blueprints/Player/BP_PlayerController.CreateWidget` (`self.PlayerController`) "/Game/Blueprints/UI/BP_HUD.BP_HUD_C"))
  (bind _asbp_hud (cast `/Game/Blueprints/UI/BP_HUD` _result))
  (bind _output_get (set `self.HUD` _asbp_hud))
  (set `/Game/Blueprints/GameStateMachine/BP_GameStateMachine.HUD` _output_get (`self.GameStateMachine`)))

(fn `OnEnter`
  (`parent.OnEnter`)
  (`UserWidget.AddToPlayerScreen` (`self.HUD`) 0))

(fn `OnExit`
  (`parent.OnExit`)
  (`Widget.RemoveFromParent` (`self.HUD`)))

(fn `OnTick`
  (params (InDeltaTime :type "Float (double-precision)"))
  (`parent.OnTick` 0.0))
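; Game mode that owns and drives the game's state machine and tracks elapsed game time.
; When the level-began event is raised, it caches the player character and controller, printing errors if missing, and passes them to a newly constructed BP_GameStateMachine.
; Tick forwards delta time to that machine.
; It also exposes the state machine and camera manager through accessors; its player-spawn logic is unconnected.
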(event `self.ReceiveBeginPlay`)

(event `/Game/Blueprints/Core/Interfaces/BPI_OnLevelBeginedSubscriber.OnLevelBeginedRaised`
  (`self.SetPlayerVariables`)
  (`self.ConstructStateMachine`))

(event `self.ReceiveTick`
  (params (DeltaSeconds :type "Float (single-precision)"))
  (set `self.GameTime` (+ DeltaSeconds (`self.GameTime`)))
  (`/Game/Blueprints/StatePatter/BP_StateMachineBase.OnTick` (`self.GameStateMachine`) DeltaSeconds))

(fn `ConstructStateMachine`
  (bind _returnvalue (`|GenericCreateObject` "/Game/Blueprints/GameStateMachine/BP_GameStateMachine.BP_GameStateMachine_C" (`self.PlayerCharacter`) (`self.PlayerController`)))
  (bind _output_get (set `self.GameStateMachine` _returnvalue))
  (`/Game/Blueprints/StatePatter/BP_StateMachineBase.Init` _output_get))

(fn `GetCameraManager`
  (returns (CameraManager :type "/Game/Blueprints/Camera/BP_CameraManager Object Reference"))
  (return (`self.CameraManager`)))

(fn `GetGameStateMachine`
  (returns (GameStateMachine :type "/Game/Blueprints/GameStateMachine/BP_GameStateMachine Object Reference"))
  (return (`self.GameStateMachine`)))

(fn `SetCameraManager`
  (params (CameraManager :type "/Game/Blueprints/Camera/BP_CameraManager Object Reference"))
  (set `self.CameraManager` CameraManager)
  (return))

(fn `SetPlayerVariables`
  ;[1 1 1] PlayerCharacter
  (bind _asbp_third_person_character (cast `/Game/Blueprints/Player/BP_ThirdPersonCharacter` (`GameplayStatics.GetPlayerCharacter` 0))
    (:`then`
      (bind _output_get (set `self.PlayerCharacter` _asbp_third_person_character))
      (`/Engine/EditorBlueprintResources/StandardMacros.IsValid` _output_get
        (:`Is Valid`
          _)
        (:`Is Not Valid`
          (`KismetSystemLibrary.PrintString` "No player Character" true true (struct :`R` 1.0 :`A` 1.0) :!label _label))))
    (:`CastFailed`
      (goto _label)))
  ;[1 1 1] PlayerController
  (bind _asbp_player_controller (cast `/Game/Blueprints/Player/BP_PlayerController` (`GameplayStatics.GetPlayerController` 0))
    (:`then`
      (bind _output_get_2 (set `self.PlayerController` _asbp_player_controller))
      (`/Engine/EditorBlueprintResources/StandardMacros.IsValid` _output_get_2
        (:`Is Not Valid`
          _)))
    (:`CastFailed`
      _))
  (`KismetSystemLibrary.PrintString` "No player controller" true true (struct :`R` 1.0 :`A` 1.0)))

(fn `UserConstructionScript`)
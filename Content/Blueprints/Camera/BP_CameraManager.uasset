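; Camera manager actor that owns an on-spline camera plus camera-path and look-at splines as child actors, and hands their control to a state machine.
; A guarded Init caches game instance, game mode, player and child-actor references, then registers the manager with the game mode.
; OnLevelBeginedRaised constructs and initializes BP_CameraStateMachine with those references.
; Tick forwards delta time to the state machine, which holds the camera logic.
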(event `self.ReceiveBeginPlay`
  (if (not (`self.Inited`))
    (`self.Init`)))

(event `/Game/Blueprints/Core/Interfaces/BPI_Initiable.Init`
  (if (not (`self.Inited`))
    (set `self.Inited` true)
    ;[1 1 1] Get game instance
    (bind _asbp_game_instance (`/Game/Blueprints/Core/BP_CastUtils.GetBP_GameInstance` self))
    (set `self.BP_GameInstance` _asbp_game_instance)
    ;[1 1 1] Get Dependencies
    (bind _asbp_third_person_game_mode (`/Game/Blueprints/Core/BP_CastUtils.GetBP_GameMode` self))
    (set `self.Game Mode` _asbp_third_person_game_mode)
    (`self.SetPlayerControllerReference`)
    (bind _ascamera_actor (cast `CameraActor` (`ChildActorComponent.ChildActor` (`self.BP_OnSplineCamera`))))
    (set `self.MainCamera` _ascamera_actor)
    (`/Game/Blueprints/BP_GameMode.SetCameraManager` (`self.Game Mode`) self)
    (set `self.PlayerCharacter` (`GameplayStatics.GetPlayerCharacter` 0))
    (`self.SetSpliesVariables`)))

(event `/Game/Blueprints/Core/Interfaces/BPI_OnLevelBeginedSubscriber.OnLevelBeginedRaised`
  ;[1 1 1] Construct state machine
  (bind _returnvalue (`|GenericCreateObject` "/Game/Blueprints/Camera/States/BP_CameraStateMachine.BP_CameraStateMachine_C" (`self.MainCamera`) (`self.Camera Spline`) (`self.Look At Camera Spline`) self (`self.PlayerController`) (`self.PlayerCharacter`)))
  (bind _output_get (set `self.CameraStateMachine` _returnvalue))
  (`/Game/Blueprints/StatePatter/BP_StateMachineBase.Init` _output_get))

(event `self.ReceiveTick`
  (params (DeltaSeconds :type "Float (single-precision)"))
  ;[1 1 1] Tick State Machine
  (bind _camerastatemachine (`self.CameraStateMachine`)
    (:`then`
      (`/Game/Blueprints/StatePatter/BP_StateMachineBase.OnTick` _camerastatemachine DeltaSeconds))
    (:`else`)))

(fn `GetInited`
  (returns (Inited :type Boolean))
  (return (`self.Inited`)))

(fn `SetPlayerControllerReference`
  (bind _returnvalue (`GameplayStatics.GetPlayerController` 0))
  (bind _debug (`self.Debug`))
  (`/Engine/EditorBlueprintResources/StandardMacros.IsValid` _returnvalue
    (:`Is Valid`
      (if _debug
        (`KismetSystemLibrary.PrintString` "Player Controller is valid"))
      (bind _asbp_player_controller (cast `/Game/Blueprints/Player/BP_PlayerController` _returnvalue))
      (set `self.PlayerController` _asbp_player_controller))
    (:`Is Not Valid`
      (if _debug
        (`KismetSystemLibrary.PrintString` "Player Controller is not valid" true true (struct :`R` 0.999 :`A` 1.0)))))
  (return))

(fn `SetSpliesVariables`
  (cast `/Game/Blueprints/Camera/BP_Camera` (`ChildActorComponent.ChildActor` (`self.BP_OnSplineCamera`)))
  (bind _asbp_camera_spline (cast `/Game/Blueprints/Camera/BP_CameraSpline` (`ChildActorComponent.ChildActor` (`self.BP_CameraSpline`))))
  (set `self.Camera Spline` _asbp_camera_spline)
  (bind _asbp_camera_spline_2 (cast `/Game/Blueprints/Camera/BP_CameraSpline` (`ChildActorComponent.ChildActor` (`self.BP_LookAtSpline`))))
  (set `self.Look At Camera Spline` _asbp_camera_spline_2)
  (return))

(fn `UserConstructionScript`)
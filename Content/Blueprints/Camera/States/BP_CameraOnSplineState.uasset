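; Camera state that moves the camera along a camera spline while it faces the point on a look-at spline nearest the player.
; On entry it makes the camera the view target.
; Each tick it offsets the player's position along the look-at spline's right vector by the horizontal player-to-camera distance, then projects that onto the camera spline.
; Position lerps and rotation quaternion-slerps toward their targets, using camera manager rates scaled by delta time.
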(fn `GetCameraTargetPosition`
  (returns (TargetCameraPosition :type "Vector Structure"))
  (bind _vector (`self.GetPlayerSameHeight`))
  (return (+ _vector (* (`self.RightSplineVector`) (`KismetMathLibrary.Vector_Distance` _vector (`Actor.K2_GetActorLocation` (`self.CameraActor`)))))))

(fn `GetLookAtPoint`
  (returns (LookAtPoint :type "Vector Structure"))
  (return (`SplineComponent.FindLocationClosestToWorldLocation` (`/Game/Blueprints/Camera/BP_CameraSpline.Spline` (`self.LookAtSpline`)) (`Actor.K2_GetActorLocation` (`self.PlayerCharacter`)) "World")))

(fn `GetPlayerSameHeight`
  (returns (Vector :type "Vector Structure"))
  (bind (_returnvalue_x _returnvalue_y) (`KismetMathLibrary.BreakVector` (`Actor.K2_GetActorLocation` (`self.PlayerCharacter`))))
  (return (`KismetMathLibrary.MakeVector` _returnvalue_x _returnvalue_y (.z (`Actor.K2_GetActorLocation` (`self.CameraActor`))))))

(fn `GetSplineDistance`
  (params (InLocation :type "Vector Structure (by ref)"))
  (returns (SplineDistance :type "Float (single-precision)"))
  (return (`SplineComponent.GetDistanceAlongSplineAtLocation` (`/Game/Blueprints/Camera/BP_CameraSpline.Spline` (`self.CameraSpline`)) InLocation "World")))

(fn `Init`
  (`parent.Init`))

(fn `OnEnter`
  (`parent.OnEnter`)
  (set `self.CurrentLocation` (`Actor.K2_GetActorLocation` (`self.CameraActor`)))
  (bind _lookatpoint (`self.GetLookAtPoint`))
  (set `self.Look at Point` _lookatpoint)
  (`/Game/Blueprints/Player/BP_PlayerController.SetTargetView` (`self.PlayerController`) (`self.CameraActor`) 0.0 "VTBlend_Linear" 0.0 false))

(fn `OnTick`
  (params (InDeltaTime :type "Float (double-precision)"))
  (returns (DeltaTime :type "Float (double-precision)"))
  (locals (DeltaSeconds :type "Float (double-precision)" :default 0.0))
  (bind _deltatime (`parent.OnTick` InDeltaTime))
  (set `local.DeltaSeconds` _deltatime)
  (bind _returnvalue (`/Game/Blueprints/Camera/BP_CameraSpline.GetRightSplineVector` (`self.LookAtSpline`) (`self.Look at Point`)))
  (set `self.RightSplineVector` _returnvalue)
  (`self.UpdateLocation` (`local.DeltaSeconds`))
  (`self.UpdateRotation` (`local.DeltaSeconds`))
  (return (`local.DeltaSeconds`)))

(fn `UpdateLocation`
  (params (DeltaSecond :type "Float (double-precision)"))
  (locals (TargetSplineDistance :type "Float (single-precision)" :default 0.0) (TargetLocation :type "Vector Structure" :default (0.0 0.0 0.0)) (DeltaSeconds :type "Float (double-precision)"))
  (set `local.DeltaSeconds` DeltaSecond)
  (bind _targetcameraposition (`self.GetCameraTargetPosition`))
  (bind _splinedistance (`self.GetSplineDistance` _targetcameraposition))
  (set `local.TargetSplineDistance` _splinedistance)
  (set `local.TargetLocation` (`SplineComponent.GetLocationAtDistanceAlongSpline` (`/Game/Blueprints/Camera/BP_CameraSpline.Spline` (`self.CameraSpline`)) (`local.TargetSplineDistance`) "World"))
  (bind _output_get (set `self.CurrentLocation` (`KismetMathLibrary.VLerp` (`self.CurrentLocation`) (`local.TargetLocation`) (`KismetMathLibrary.FClamp` (* (`/Game/Blueprints/Camera/BP_CameraManager.CameraMovementLerpParam` (`self.CameraManagera`)) (`local.DeltaSeconds`))))))
  (`Actor.K2_SetActorLocation` (`self.CameraActor`) _output_get false false)
  (return))

(fn `UpdateRotation`
  (params (DeltaSeconds :type "Float (double-precision)"))
  (locals (`Delta Time` :type "Float (double-precision)"))
  (bind _lookatpoint (`self.GetLookAtPoint`))
  (bind _output_get (set `self.Look at Point` _lookatpoint))
  (`Actor.K2_SetActorRotation` (`self.CameraActor`) (`KismetMathLibrary.Quat_Rotator` (`KismetMathLibrary.Quat_Slerp` (`KismetMathLibrary.Conv_RotatorToQuaternion` (`Actor.K2_GetActorRotation` (`self.CameraActor`))) (`KismetMathLibrary.Conv_RotatorToQuaternion` (`KismetMathLibrary.MakeRotFromX` (`KismetMathLibrary.Normal` (- _output_get (`Actor.K2_GetActorLocation` (`self.CameraActor`)))))) (* (`local.DeltaSeconds`) (`/Game/Blueprints/Camera/BP_CameraManager.CameraRotationSLerpParameter` (`self.CameraManagera`))))) false)
  (return))
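; BP_CameraStateMachine is the state machine that drives the camera, starting it in a spline-based state.
; On Init it runs the parent setup, then constructs a BP_CameraOnSplineState with references to the camera actor, camera and look-at splines, player controller, character and camera manager.
; It stores and initializes that state, then makes it current; no other states or transitions are defined here.
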(fn `Init`
  (`parent.Init`)
  (bind _returnvalue (`|GenericCreateObject` "/Game/Blueprints/Camera/States/BP_CameraOnSplineState.BP_CameraOnSplineState_C" (`self.CameraActor`) (`self.CameraSpline`) (`self.LookAtSpline`) (`self.PlayerController`) (`self.PlayerCharacter`) (`self.CameraManager`)))
  (bind _output_get (set `self.CameraOnSplineState` _returnvalue))
  (`/Game/Blueprints/StatePatter/BP_StateBase.Init` _output_get)
  (`self.SetCurrentState` _output_get))
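; BP_CameraSpline is a camera spline Blueprint that supplies world-space direction vectors along its Spline component for a given location.
; The forward vector is the spline direction at the distance along the spline corresponding to that location.
; The right vector is the cross product of world up and forward, and the left vector is its negation.
; It has no active event or construction logic.
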(fn `GetForwardSplineVectorAt`
  (params (InLocation :type "Vector Structure (by ref)"))
  (returns (`Vector Forwars` :type "Vector Structure"))
  (bind _spline (`self.Spline`))
  (return (`SplineComponent.GetDirectionAtDistanceAlongSpline` _spline (`SplineComponent.GetDistanceAlongSplineAtLocation` _spline InLocation "World") "World")))

(fn `GetLeftSplineVectorAt`
  (params (InLocation :type "Vector Structure (by ref)"))
  (returns (`Vector Left` :type "Vector Structure"))
  (bind _vector_forwars (`self.GetForwardSplineVectorAt` InLocation))
  (return (`KismetMathLibrary.NegateVector` (`KismetMathLibrary.Cross_VectorVector` (`KismetMathLibrary.Vector_Up`) _vector_forwars))))

(fn `GetRightSplineVector`
  (params (InLocation :type "Vector Structure (by ref)"))
  (returns (ReturnValue :type "Vector Structure"))
  (bind _vector_forwars (`self.GetForwardSplineVectorAt` InLocation))
  (return (`KismetMathLibrary.Cross_VectorVector` (`KismetMathLibrary.Vector_Up`) _vector_forwars)))

(fn `UserConstructionScript`)
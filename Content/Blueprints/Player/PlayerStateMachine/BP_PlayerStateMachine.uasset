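; Player state machine for the third-person character, owning and switching between Locomotion, Attack and Dodge states.
; Init constructs the state objects and starts in Locomotion, while SetCurrentStateByEnum maps an enum to each instance.
; The character's attack event passes direction and strength to the Attack state and switches to it unless already attacking; dodging blocks the switch.
; The move input is bound but its handler is empty.
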(event `self.InitEvent_Event`
  (`parent.InitEvent_Event`)
  (add `/Game/Blueprints/Player/BP_ThirdPersonCharacter.IA_Move` (`self.BP_ThirdPersonCharacter`) (delegate `IA_Move_Event`))
  (add `/Game/Blueprints/Player/BP_ThirdPersonCharacter.On_Attack` (`self.BP_ThirdPersonCharacter`) (delegate `OnAttack_Event`)))

(event `IA_Move_Event`
  (params (ActionValueX :type "Float (double-precision)") (ActionValueY :type "Float (double-precision)") (InputAction :type "InputAction Object Reference")))

(event `OnAttack_Event`
  (params (AttackDirection :type "/Game/Blueprints/Player/PlayerStateMachine/BPE_AttackDirection Enum" :default "NewEnumerator0") (IsStrong :type Boolean))
  (bind _attackstate (`self.AttackState`))
  (bind _currentstate (`self.GetCurrentState`))
  (if (!= _currentstate (`self.AttackState`))
    (set `/Game/Blueprints/Player/PlayerStateMachine/BP_AttackPlayerState.AttackDirection` AttackDirection _attackstate)
    (set `/Game/Blueprints/Player/PlayerStateMachine/BP_AttackPlayerState.IsStrongAttack` IsStrong _attackstate)
    (bind _currentstate_2 (`self.GetCurrentState`))
    (if (!= _currentstate_2 (`self.DodgeState`))
      (`self.SetCurrentStateByEnum` "NewEnumerator1"))))

(fn `Init`
  (bind _returnvalue (`|GenericCreateObject` "/Game/Blueprints/Player/PlayerStateMachine/BP_LocomotionPlayerStateState.BP_LocomotionPlayerStateState_C" self (`self.BP_ThirdPersonCharacter`)))
  (`/Game/Blueprints/StatePatter/BP_StateBase.Init` _returnvalue)
  (bind _output_get (set `self.LocomotionState` _returnvalue))
  (`self.SetCurrentState` _output_get)
  (bind _returnvalue_2 (`|GenericCreateObject` "/Game/Blueprints/Player/PlayerStateMachine/BP_AttackPlayerState.BP_AttackPlayerState_C" "NewEnumerator0" (`self.BP_ThirdPersonCharacter`) self))
  (`/Game/Blueprints/StatePatter/BP_StateBase.Init` _returnvalue_2)
  (set `self.AttackState` _returnvalue_2)
  (bind _returnvalue_3 (`|GenericCreateObject` "/Game/Blueprints/Player/PlayerStateMachine/BP_DodgePlayerState.BP_DodgePlayerState_C" (`self.BP_ThirdPersonCharacter`)))
  (set `self.DodgeState` _returnvalue_3)
  (`parent.Init`))

(fn `SetCurrentStateByEnum`
  (params (PlayerState :type "/Game/Blueprints/Player/PlayerStateMachine/BPE_PlayerState Enum" :default "NewEnumerator0"))
  (switch `/Game/Blueprints/Player/PlayerStateMachine/BPE_PlayerState` PlayerState
    (:`NewEnumerator0`
      (`self.SetCurrentState` (`self.LocomotionState`)))
    (:`NewEnumerator1`
      (`self.SetCurrentState` (`self.AttackState`)))
    (:`NewEnumerator2`
      (`self.SetCurrentState` (`self.DodgeState`)))))
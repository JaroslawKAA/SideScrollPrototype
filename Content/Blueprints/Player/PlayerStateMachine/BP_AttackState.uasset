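; Player state machine state that runs a normal or strong left/right attack.
; On enter it sets the anim instance's attack flags, rotates the character toward the attack direction and updates the attack target state if a close enemy is valid.
; A tick timer switches the state machine to another state once the queried animation length elapses.
; Exit clears the attack flag and sets the target state again.
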(fn `Init`
  (`parent.Init`)
  (set `self.Anim Instance` (`/Game/Blueprints/Core/BP_CharacterBase.AnimInstance` (`self.PlayerCharacter`))))

(fn `OnEnter`
  (bind _playercharacter (`self.PlayerCharacter`))
  (`parent.OnEnter`)
  (`/Game/Characters/Mannequins/Animations/ABP_Manny.SetAttack` (`/Game/Blueprints/Core/BP_CharacterBase.AnimInstance` (`self.PlayerCharacter`)) true (`self.IsStrongAttack`) (`self.AttackDirection`))
  (set `self.AnimationTimer` 0.0)
  (bind _second (`/Game/Characters/Mannequins/Animations/ABP_Manny.GetAttackAnimationLenght` (`self.Anim Instance`) (`self.IsStrongAttack`) (`self.AttackDirection`)))
  (set `self.AttackAnimationLenght` _second)
  (switch `/Game/Blueprints/Player/PlayerStateMachine/BPE_AttackDirection` (`self.AttackDirection`)
    (:`NewEnumerator0`
      (`/Game/Blueprints/Player/BP_ThirdPersonCharacter.Rotate Left` _playercharacter))
    (:`NewEnumerator1`
      (`/Game/Blueprints/Player/BP_ThirdPersonCharacter.RotateRight` _playercharacter)))
  (`/Engine/EditorBlueprintResources/StandardMacros.IsValid` (`/Game/Blueprints/Player/BP_ThirdPersonCharacter.CloseEnemy` (`self.PlayerCharacter`))
    (:`Is Valid`
      (set `/Game/Blueprints/Core/BP_CharacterBase.m_AttackTargetState` "NewEnumerator0" (`self.PlayerCharacter`)))))

(fn `OnExit`
  (`parent.OnExit`)
  (set `/Game/Characters/Mannequins/Animations/ABP_Manny.IsAttack` false (`/Game/Blueprints/Core/BP_CharacterBase.AnimInstance` (`self.PlayerCharacter`)))
  (set `/Game/Blueprints/Core/BP_CharacterBase.m_AttackTargetState` "NewEnumerator1" (`self.PlayerCharacter`)))

(fn `OnTick`
  (params (InDeltaTime :type "Float (double-precision)"))
  (`parent.OnTick` InDeltaTime)
  (set `self.AnimationTimer` (+ (`self.AnimationTimer`) (`local.InDeltaTime`)))
  (if (> (`self.AnimationTimer`) (`self.AttackAnimationLenght`))
    (`/Game/Blueprints/Player/PlayerStateMachine/BP_PlayerStateMachine.SetCurrentStateByEnum` (`self.PlayerStateMachine`) "NewEnumerator0")))
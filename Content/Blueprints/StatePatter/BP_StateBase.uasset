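; BP_StateBase is a base class for states in a state pattern, defining the Init, OnEnter, OnTick and OnExit lifecycle.
; Init caches the class display name and calls an init event, whose handler in the event graph is empty.
; OnEnter prints that name as a debug message, while OnTick only passes delta time through and OnExit is empty.
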(event `InitEvent_Event`)

(fn `Init`
  (set `self.ClassName` (`KismetSystemLibrary.GetClassDisplayName` (`GameplayStatics.GetObjectClass` self)))
  (`self.InitEvent_Event`)
  (return))

(fn `OnEnter`
  (`KismetSystemLibrary.PrintString` null (`KismetStringLibrary.Concat_StrStr` "On Enter State: " (`self.ClassName`)))
  (return))

(fn `OnExit`
  (return))

(fn `OnTick`
  (params (InDeltaTime :type "Float (double-precision)"))
  (returns (DeltaTime :type "Float (double-precision)"))
  (return InDeltaTime))
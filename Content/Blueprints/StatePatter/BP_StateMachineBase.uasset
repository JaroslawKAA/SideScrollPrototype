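; BP_StateMachineBase is a base state machine Blueprint for a State pattern, holding a single current state object.
; SetCurrentState calls OnExit on the old state, stores the new one, calls OnEnter on it and fires a state-changed event.
; OnTick forwards delta time to the current state when valid, and Init fires an init event.
; Both event handlers in the event graph are empty.
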(event `OnStateChanged_Event`
  (params (State :type "/Game/Blueprints/StatePatter/BP_StateBase Object Reference")))

(event `InitEvent_Event`)

(fn `GetCurrentState`
  (returns (CurrentState :type "/Game/Blueprints/StatePatter/BP_StateBase Object Reference"))
  (return (`self.CurrentState`)))

(fn `Init`
  (`self.InitEvent_Event`)
  (return))

(fn `OnTick`
  (params (InDeltaTime :type "Float (double-precision)"))
  (returns (DeltaTime :type "Float (double-precision)"))
  (bind _currentstate (`self.CurrentState`)
    (:`then`
      (`/Game/Blueprints/StatePatter/BP_StateBase.OnTick` _currentstate InDeltaTime)
      (return InDeltaTime))
    (:`else`)))

(fn `SetCurrentState`
  (params (NewState :type "/Game/Blueprints/StatePatter/BP_StateBase Object Reference"))
  ;[1 1 1] Exit previous state
  (bind _currentstate (`self.CurrentState`)
    (:`then`
      (`/Game/Blueprints/StatePatter/BP_StateBase.OnExit` _currentstate))
    (:`else`
      _))
  (bind _output_get (set `self.CurrentState` NewState))
  ;[1 1 1] Enter new state
  (`/Engine/EditorBlueprintResources/StandardMacros.IsValid` _output_get
    (:`Is Valid`
      (`/Game/Blueprints/StatePatter/BP_StateBase.OnEnter` (`self.CurrentState`)))
    (:`Is Not Valid`
      _))
  (`self.OnStateChanged_Event` (`self.CurrentState`))
  (return))